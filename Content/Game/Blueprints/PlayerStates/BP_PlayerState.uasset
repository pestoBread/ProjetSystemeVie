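; Player state that owns the player's health component and keeps health persistent through the game instance.
; On BeginPlay it either restores saved current and max health from BP_GameInstance or resets health and flags it as initialized.
; Health change events write both values back to the game instance.
; On death it asks BP_ThirdPersonGameMode to start respawning player controller 0.
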(event `self.ReceiveBeginPlay`
  (bind _asbp_game_instance (cast `/Game/Game/Blueprints/BP_GameInstance` (`GameplayStatics.GetGameInstance`)))
  (bind _output_get (set `self.As BP Game Instance` _asbp_game_instance))
  (if (`/Game/Game/Blueprints/BP_GameInstance.HealthInitialized_GI` _output_get)
    (`self.LoadHealthFromGI`)
    (else
      (`/Game/Game/Blueprints/Interfaces/BPI_Damageable.ResetHealth` (`self.AC_Health`))
      (set `/Game/Game/Blueprints/BP_GameInstance.HealthInitialized_GI` true (`self.As BP Game Instance`)))))

(event `self.AC_Health.OnHealthChanged`
  (params (CurrentHealth :type "Float (double-precision)") (MaxHealth :type "Float (double-precision)"))
  (`self.SetCurrentHealth` CurrentHealth)
  (`self.SetMaxHealth` MaxHealth))

(event `self.AC_Health.OnDeath`
  (bind _asbp_third_person_game_mode (cast `/Game/Game/Blueprints/GameModes/BP_ThirdPersonGameMode` (`GameplayStatics.GetGameMode`)))
  (`/Game/Game/Blueprints/GameModes/BP_ThirdPersonGameMode.StartRespawn` _asbp_third_person_game_mode (`GameplayStatics.GetPlayerController` 0)))

(fn `LoadHealthFromGI`
  (bind _as_bp_game_instance (`self.As BP Game Instance`))
  (bind _ac_health (`self.AC_Health`))
  (bind _output_get (set `/Game/Game/Blueprints/Components/AC_Health.MaxHealth` (`/Game/Game/Blueprints/BP_GameInstance.MaxHealth_GI` _as_bp_game_instance) _ac_health))
  (bind _output_get_2 (set `/Game/Game/Blueprints/Components/AC_Health.CurrentHealth` (`/Game/Game/Blueprints/BP_GameInstance.CurrentHealth_GI` _as_bp_game_instance) _ac_health))
  (`/Game/Game/Blueprints/Components/AC_Health.OnHealthChanged` _ac_health _output_get_2 _output_get))

(fn `SetCurrentHealth`
  (params (NewHealth :type "Float (double-precision)"))
  (set `/Game/Game/Blueprints/BP_GameInstance.CurrentHealth_GI` NewHealth (`self.As BP Game Instance`)))

(fn `SetMaxHealth`
  (params (NewMaxHealth :type "Float (double-precision)"))
  (set `/Game/Game/Blueprints/BP_GameInstance.MaxHealth_GI` NewMaxHealth (`self.As BP Game Instance`)))

(fn `UserConstructionScript`)