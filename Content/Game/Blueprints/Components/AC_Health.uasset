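; AC_Health is a health component that tracks current health and dead state for its owner.
; UpdateHealth adds a signed amount unless dead, and ResetHealth revives the owner at max health.
; Both route through UpdateHealthAndNotify, which clamps the value, broadcasts OnHealthChanged, and at zero sets IsDead and broadcasts OnDeath.
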(event `/Game/Game/Blueprints/Interfaces/BPI_Damageable.UpdateHealth`
  (params (Amount :type "Float (double-precision)"))
  (if (not (`self.IsDead`))
    (`self.UpdateHealthAndNotify` (+ Amount (`self.CurrentHealth`)))))

(event `/Game/Game/Blueprints/Interfaces/BPI_Damageable.ResetHealth`
  (set `self.IsDead` false)
  (`self.UpdateHealthAndNotify` (`self.MaxHealth`)))

(fn `UpdateHealthAndNotify`
  (params (NewHealthValue :type "Float (double-precision)"))
  (bind _output_get (set `self.CurrentHealth` (`KismetMathLibrary.FClamp` NewHealthValue 0.0 (`self.MaxHealth`))))
  (`self.OnHealthChanged` _output_get (`self.MaxHealth`))
  (if (<= _output_get 0.0)
    (set `self.IsDead` true)
    (`self.OnDeath`)))